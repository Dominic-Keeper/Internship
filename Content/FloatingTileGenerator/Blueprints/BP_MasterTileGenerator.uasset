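; BP_MasterTileGenerator builds a grid of instanced mesh tiles, spaced by mesh bounds plus padding, with optional height steps along X or Y.
; Its construction script either generates and stores tile transforms, or rebuilds instances from them with optional random rotation jitter.
; When rebuilding, it also pushes debug, lerp, idle-rotation and optional randomization settings to every BP_InstanceMover referencing it.
; Boolean flags act as one-shot editor buttons that reset after running.
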(fn `UserConstructionScript`
  (bind _returnvalue (`KismetMathLibrary.RandomFloatInRange` -2.0 2.0))
  (bind _tiletransform (`self.TileTransform`))
  (bind _tiletransform_2 (`self.TileTransform`))
  ;[1 1 1] Add instance static mesh for tiles and set instance mesh
  (bind _returnvalue_2 (`AddComponent|InstancedStaticMeshComponent_0`))
  (bind _output_get (set `self.TileInstance` _returnvalue_2))
  (`StaticMeshComponent.SetStaticMesh` _output_get (`self.InstanceMesh`))
  (bind (_min _max) (`StaticMeshComponent.GetLocalBounds` _output_get))
  ;[1 1 1] Get mesh bounds and add padding
  (set `self.TileBoundsX` (+ (- (.x _max) (.x _min)) (`self.PaddingX`)))
  (set `self.TileBoundsY` (+ (- (.y _max) (.y _min)) (`self.PaddingY`)))
  (if (`self.GenerateGrid`)
    ;[1 1 1] Generate Grid
    (`KismetArrayLibrary.Array_Clear` (`self.TileTransform`))
    (for _index (range (* (`self.GridSizeX`) (`self.GridSizeY`)))
      (bind (_x _y) (`self.IndexToSquareGridLocation` _index) ; Converts grid index to tiles location.
        (:`  `
          (`KismetArrayLibrary.Array_Add` _tiletransform (`KismetMathLibrary.MakeTransform` (`KismetMathLibrary.MakeVector` _x _y (select `bool` (`self.X_Or_Y_Step`) :`false` (* (/ _x (`self.TileBoundsX`)) (`self.StepHight`)) :`true` (* (/ _y (`self.TileBoundsY`)) (`self.StepHight`))))))
          (`InstancedStaticMeshComponent.AddInstance` (`self.TileInstance`) (`KismetArrayLibrary.Array_Get` _tiletransform _index)))))
    (set `self.GenerateGrid` false)
    (else
      ;[1 1 1] Recreate grid from genarated transform array
      (for (_array_element _array_index) _tiletransform_2
        (bind _item (`KismetArrayLibrary.Array_Get` _tiletransform_2 _array_index))
        (`KismetArrayLibrary.Array_Set` _tiletransform_2 _array_index (`KismetMathLibrary.MakeTransform` (.location _array_element) (select `bool` (`self.RandomTileRotation`) :`false` (.rotation _array_element) :`true` (`KismetMathLibrary.ComposeRotators` (.rotation _array_element) (`KismetMathLibrary.MakeRotator` (+ (.roll (.rotation _item)) _returnvalue) (+ (.pitch (.rotation _item)) _returnvalue) (+ (.yaw (.rotation _item)) _returnvalue)))) (.scale _array_element)))
        (`InstancedStaticMeshComponent.AddInstance` (`self.TileInstance`) (`KismetArrayLibrary.Array_Get` _tiletransform_2 _array_index)))
      (set `self.RandomTileRotation` false) ; Switch off add rotation
      ;[1 1 1] Update  BP_InstanceMovers attached
      (bind _outactors (`GameplayStatics.GetAllActorsOfClass` "/Game/FloatingTileGenerator/Blueprints/BP_InstanceMover.BP_InstanceMover_C"))
      (for _array_element_2 _outactors
        (if (== (`/Game/FloatingTileGenerator/Blueprints/BP_InstanceMover.MastarTileGenerator` _array_element_2) self)
          (set `/Game/FloatingTileGenerator/Blueprints/BP_InstanceMover.DebugTransform` (`self.DebugTransformer`) _array_element_2)
          (set `/Game/FloatingTileGenerator/Blueprints/BP_InstanceMover.EnableLerp` (`self.EnableMoverLerp`) _array_element_2)
          (set `/Game/FloatingTileGenerator/Blueprints/BP_InstanceMover.IdleRotating` (`self.EnableIdleRotationg`) _array_element_2)
          (if (`self.AffectMoversProperties`)
            (set `/Game/FloatingTileGenerator/Blueprints/BP_InstanceMover.MinRandomLocation` (`self.MinRandomLocation`) _array_element_2)
            (set `/Game/FloatingTileGenerator/Blueprints/BP_InstanceMover.MaxRandomLocation` (`self.MaxRandomLocation`) _array_element_2)
            (set `/Game/FloatingTileGenerator/Blueprints/BP_InstanceMover.RandomizeLocation` (`self.RandomizeLocation`) _array_element_2)
            (set `/Game/FloatingTileGenerator/Blueprints/BP_InstanceMover.RandomizeRotation` (`self.RandomizeRotation`) _array_element_2)
            (`SceneComponent.SetVisibility` (`/Game/FloatingTileGenerator/Blueprints/BP_InstanceMover.OnPlaceColision` _array_element_2) (`self.DebugColisionON`) false)
            (`SceneComponent.SetVisibility` (`/Game/FloatingTileGenerator/Blueprints/BP_InstanceMover.EnableTickColision` _array_element_2) (`self.DebugColisionON`) false)
            (`/Game/FloatingTileGenerator/Blueprints/BP_InstanceMover.Remote` _array_element_2)
            (else
              (`/Game/FloatingTileGenerator/Blueprints/BP_InstanceMover.SetTilesLocation` _array_element_2)))))
      (set `self.RandomizeLocation` false)
      (set `self.RandomizeRotation` false))))