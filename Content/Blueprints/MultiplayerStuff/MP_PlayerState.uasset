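; Multiplayer PlayerState that pushes each player's name onto a Name_HPBar widget.
; UpdateUserNames writes PlayerName to a cached bar; if none is valid, it takes one from the NameHP component on player controller 0's TopDownCharacter, flagged in-file as likely the wrong controller.
; ForceUpdateAllNames runs that update on every MP_PlayerState in the GameState's PlayerArray, with debug prints throughout.
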(event `self.ReceiveBeginPlay`)

(event `self.ReceiveTick`
  (params (DeltaSeconds :type "Float (single-precision)")))

(fn `forceUpdateAllNames`
  (bind _playerarray (`GameState.PlayerArray` (`GameplayStatics.GetGameState`)))
  (for _array_element _playerarray
    (bind _asmp_player_state (cast `/Game/Blueprints/MultiplayerStuff/MP_PlayerState` _array_element)
      (:`then`
        (`self.updateUserNames` _asmp_player_state))
      (:`CastFailed`
        (`KismetSystemLibrary.PrintString` "cast failed at playerstate" true true (struct :`G` 0.66 :`B` 1.0 :`A` 1.0) 15.0))))
  (`KismetSystemLibrary.PrintString` (`KismetStringLibrary.Conv_IntToString` (`KismetArrayLibrary.Array_Length` _playerarray)) true true (struct :`G` 0.66 :`B` 1.0 :`A` 1.0) 10.0))

(fn `updateUserNames`
  (bind _playername (`self.PlayerName`))
  (bind _playerbar (`self.playerBar`))
  (`/Engine/EditorBlueprintResources/StandardMacros.IsValid` _playerbar
    (:`Is Valid`
      (`/Game/Blueprints/GameInfo/Name_HPBar.setUsername` _playerbar _playername)
      (`KismetSystemLibrary.PrintString` _playername true true (struct :`G` 0.66 :`B` 1.0 :`A` 1.0) 10.0))
    (:`Is Not Valid`
      (`KismetSystemLibrary.PrintString` "HUD is not valid" true true (struct :`R` 0.77 :`G` 0.497474 :`B` 0.055433 :`A` 1.0) 15.0)
      (bind _astop_down_character (cast `/Game/TopDownBP/Blueprints/TopDownCharacter` (`Controller.K2_GetPawn` (`GameplayStatics.GetPlayerController` 0)))
        (:`then`
          (bind _asname_hpbar (cast `/Game/Blueprints/GameInfo/Name_HPBar` (`WidgetComponent.GetUserWidgetObject` (`/Game/TopDownBP/Blueprints/TopDownCharacter.NameHP` _astop_down_character)))
            (:`then`
              (bind _output_get (set `self.playerBar` _asname_hpbar))
              (`/Game/Blueprints/GameInfo/Name_HPBar.setUsername` _output_get (`self.PlayerName`))
              (`KismetSystemLibrary.PrintString` "Hello"))
            (:`CastFailed`
              (`KismetSystemLibrary.PrintString` "failed HP bar" true true (struct :`R` 1.0 :`G` 0.055031 :`A` 1.0) 20.0))))
        (:`CastFailed`
          (`KismetSystemLibrary.PrintString` "Failed TopDownCast (MP_PlayerState)" true true (struct :`R` 1.0 :`G` 0.218901 :`A` 1.0) 20.0))))))

(fn `UserConstructionScript`)