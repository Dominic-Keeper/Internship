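; Game instance that holds the game's list of quests and provides lookups into it by ID.
; Init seeds the Quests array with a single example quest.
; GetQuestByID and GetQuestStatusByID scan the array linearly for a matching ID, returning the quest or its status.
; The status lookup returns -1 when no quest matches.
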(event `self.ReceiveInit`
  (`KismetArrayLibrary.Array_Add` (`self.Quests`) (make `/Game/Blueprints/Data/Quest` 100 "ExampleQuest" 1)))

(fn `GetQuestByID`
  (params (ID :type Integer))
  (returns (Quest :type "/Game/Blueprints/Data/Quest Structure"))
  (for _array_element (`self.Quests`)
    (if (== (`.ID_3_92D620FB46C24E5829F34A8BEA7EF777` (break `/Game/Blueprints/Data/Quest` _array_element)) ID)
      (return _array_element)))
  (return))

(fn `GetQuestStatusByID`
  (params (ID :type Integer))
  (returns (Status :type Integer))
  (for _array_element (`self.Quests`)
    (bind (_id _name _status) (break `/Game/Blueprints/Data/Quest` _array_element))
    (if (== _id ID)
      (return _status)))
  (return -1))