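; WorldObject is an actor set up for adjustable opacity on its static meshes.
; Its construction script walks child components to create dynamic material instances, store them and assign them to slot 0, but no parent material is wired and the function returns within the first iteration.
; ChangeMatTransparency sets Opacity on new instances made from each passed material's parent, without assigning them to meshes.
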(event `self.ReceiveBeginPlay`)

(fn `changeMatTransparency`
  (params (InstancedMaterials :type "Array of MaterialInstanceDynamic Object Reference") (Opacity :type "Float (double-precision)"))
  (for (_array_element _array_index) InstancedMaterials
    (bind _returnvalue (`KismetMaterialLibrary.CreateDynamicMaterialInstance` _array_element (`MaterialInstance.Parent` (`KismetArrayLibrary.Array_Get` InstancedMaterials _array_index))))
    (`MaterialInstanceDynamic.SetScalarParameterValue` _returnvalue "Opacity" Opacity)))

(fn `CreateInstancedMaterials`
  (for _array_element (`SceneComponent.GetChildrenComponents` (`self.DefaultSceneRoot`) true)
    (bind _asstatic_mesh_component (cast `StaticMeshComponent` _array_element)
      (:`then`
        (for _array_element_2 (`MeshComponent.GetMaterials` _asstatic_mesh_component)
          (bind _returnvalue (`KismetMaterialLibrary.CreateDynamicMaterialInstance` _array_element_2))
          (`KismetArrayLibrary.Array_Add` (`self.instancedMaterials`) _returnvalue)
          (`PrimitiveComponent.SetMaterial` _asstatic_mesh_component 0 _returnvalue)
          (return)))
      (:`CastFailed`
        (`KismetSystemLibrary.PrintString` "GG")
        (return))))
  (return))

(fn `UserConstructionScript`
  (`self.CreateInstancedMaterials`))