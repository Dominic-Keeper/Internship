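; Interactable character that follows whoever interacts with it, as a toggle between following and stopping.
; On the server, an interaction either sets the followed actor or clears it and stops movement.
; Authority-only Tick issues an AI MoveTo toward the followed actor within a follow distance, using a Moving flag intended to guard against repeat requests.
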(event `OnInteraction`
  (params (InteractingController :type "Controller Object Reference") (InteractingActor :type "Actor Object Reference"))
  (`/Engine/EditorBlueprintResources/ActorMacros.Switch Has Authority`
    (:`Authority`
      ;[1 1 1] Set interacting actor
      (if (== null (`self.FollowedActor`))
        (set `self.FollowedActor` null)
        (`NavMovementComponent.StopActiveMovement` (`self.CharacterMovement`))
        (set `self.Moving` false)
        (else
          (bind _output_get (set `self.FollowedActor` InteractingActor))
          (`KismetSystemLibrary.PrintString` (`KismetSystemLibrary.GetDisplayName` _output_get)))))))

(event `self.ReceiveTick`
  (params (DeltaSeconds :type "Float (single-precision)"))
  (`/Engine/EditorBlueprintResources/ActorMacros.Switch Has Authority`
    (:`Authority`
      ;[1 1 1] Check if interacting character is set
      (`/Engine/EditorBlueprintResources/StandardMacros.IsValid` (`self.FollowedActor`)
        (:`Is Valid`
          (if (not (`self.Moving`))
            (set `self.Moving` true)
            ;[1 1 1] Move to interacting character
            (`|AIMoveTo` self (0.0 0.0 0.0) (`self.FollowedActor`) (`self.FollowDistance`) true
              (:`then`
                _)
              (:`OnSuccess`
                _)
              (:`OnFail`
                _))
            (set `self.Moving` false)))))))

(fn `UserConstructionScript`)