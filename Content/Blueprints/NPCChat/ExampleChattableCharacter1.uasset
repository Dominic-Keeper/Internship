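; An example chattable NPC that offers the player a shotgun shell to the face through a short branching conversation.
; SetupNextNode switches on node ID to show dialog lines or a Yes/No choice, each naming the following node, with unhandled IDs hiding the chat.
; Accepting applies massive shot damage to the chatting controller and clears HasShotgunShell, so later requests get an out-of-shells reply.
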(event `self.SetupNextNode`
  (params (NextNodeID :type Integer))
  (switch `int` NextNodeID
    (:`Default`
      (`self.HideChat`))
    (:`0`
      (`self.ShowDialog` "Hello." 1))
    (:`1`
      (`self.ShowDialog` "Would you like a shotgun shell to the face?" 2))
    (:`2`
      (`self.ShowOptions` "Yes." "No." "" "" "" "" 3 -1))
    (:`3`
      (if (`self.HasShotgunShell`)
        (`self.ShowDialog` "Here you go!" -1)
        (`GameplayStatics.ApplyDamage` (`self.ChattingController`) 100000.0 null self "/Game/Blueprints/damageTypes/DMG_Shot.DMG_Shot_C")
        (set `self.HasShotgunShell` false)
        (else
          (`self.ShowDialog` "Damn, I'm all out of shells." -1))))))

(fn `UserConstructionScript`
  (`parent.UserConstructionScript`))