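; Base NPC character for node-based dialogue: interaction starts at node 0, and chat-continue events pass the next node ID to SetupNextNode, an empty hook.
; Helper functions show either a dialog line or up to six replies with target nodes, swapping between two lazily created widgets that reference the NPC as owner.
; PlaySound keeps one 2D chat sound playing at a time, and HideChat removes both widgets and stops it.
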(event `/Game/Blueprints/Interaction/Interactable.OnInteraction`
  (params (InteractingActor :type "Actor Object Reference"))
  (`self.SetupNextNode` 0))

(event `/Game/Blueprints/Interaction/Interactable.OnChatContinue`
  (params (NextNodeID :type Integer))
  (`self.SetupNextNode` NextNodeID))

(event `self.ReceiveBeginPlay`)

(event `self.ReceiveTick`
  (params (DeltaSeconds :type "Float (single-precision)")))

(fn `HideChat`
  ;[1 1 1] Remove interfaces
  (`Widget.RemoveFromParent` (`self.DialogBox`))
  (set `self.DialogBox` null)
  (`Widget.RemoveFromParent` (`self.OptionBox`))
  (set `self.OptionBox` null)
  ;[1 1 1] Stop effects from chat
  (`AudioComponent.Stop` (`self.CurrentChatSound`)))

(fn `PlaySound`
  (params (Sound :type "SoundBase Object Reference"))
  (bind _currentchatsound (`self.CurrentChatSound`))
  ;[1 1 1] Stop sound if there is one running
  (if (`KismetSystemLibrary.IsValid` _currentchatsound)
    (`AudioComponent.Stop` _currentchatsound))
  ;[1 1 1] Start new sound
  (bind _returnvalue (`GameplayStatics.CreateSound2D` Sound))
  (bind _output_get (set `self.CurrentChatSound` _returnvalue))
  (`AudioComponent.Play` _output_get 0.0))

(fn `SetupNextNode`
  (params (NextNodeID :type Integer)))

(fn `ShowDialog`
  (params (Text :type Text) (NodeAfter :type Integer))
  (bind _optionbox (`self.OptionBox`))
  (`|ExecutionSequence`
    (:`then_0`
      (if (== (`self.DialogBox`) null)
        (bind _returnvalue (`|CreateWidget` "/Game/Blueprints/NPCChat/Widgets/DialogBox.DialogBox_C" (`GameplayStatics.GetPlayerController` 0)))
        (`|ExecutionSequence`
          (:`then_0`
            (set `/Game/Blueprints/NPCChat/Widgets/DialogBox.OwnerActor` self _returnvalue))
          (:`then_1`
            (bind _output_get (set `self.DialogBox` _returnvalue))
            (`UserWidget.AddToViewport` _output_get 0)))))
    (:`then_1`
      ;[1 1 1] Remove ReplyBox if showing
      (if (`KismetSystemLibrary.IsValid` _optionbox)
        (`Widget.RemoveFromParent` _optionbox)
        (set `self.OptionBox` null)))
    (:`then_2`
      (`/Game/Blueprints/NPCChat/Widgets/DialogBox.SetText` (`self.DialogBox`) Text NodeAfter))))

(fn `ShowOptions`
  (params (Option1 :type Text) (Option2 :type Text) (Option3 :type Text) (Option4 :type Text) (Option5 :type Text) (Option6 :type Text) (`Option 1 Node` :type Integer) (`Option 2 Node` :type Integer) (`Option 3 Node` :type Integer) (`Option 4 Node` :type Integer) (`Option 5 Node` :type Integer) (`Option 6 Node` :type Integer))
  (bind _dialogbox (`self.DialogBox`))
  (`|ExecutionSequence`
    (:`then_0`
      (if (== (`self.OptionBox`) null)
        (bind _returnvalue (`|CreateWidget` "/Game/Blueprints/NPCChat/Widgets/ReplyBox.ReplyBox_C" (`GameplayStatics.GetPlayerController` 0)))
        (`|ExecutionSequence`
          (:`then_0`
            (set `/Game/Blueprints/NPCChat/Widgets/ReplyBox.OwnerActor` self _returnvalue))
          (:`then_1`
            (bind _output_get (set `self.OptionBox` _returnvalue))
            (`UserWidget.AddToViewport` _output_get 0)))))
    (:`then_1`
      ;[1 1 1] Remove dialog box if showing
      (if (`KismetSystemLibrary.IsValid` _dialogbox)
        (`Widget.RemoveFromParent` _dialogbox)
        (set `self.DialogBox` null)))
    (:`then_2`
      (`/Game/Blueprints/NPCChat/Widgets/ReplyBox.SetText` (`self.OptionBox`) Option1 Option2 Option3 Option4 Option5 Option6 `Option 1 Node` `Option 2 Node` `Option 3 Node` `Option 4 Node` `Option 5 Node` `Option 6 Node`))))

(fn `UserConstructionScript`)